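; BP_VaultDoor is a vault door that opens with a two-stage animation when its bound VaultOpen event fires.
; On BeginPlay it binds OpenVault to that event, and a DoOnce lets the opening run only once.
; The RotatingHandle timeline spins the handle in pitch, then on finishing starts the Opening timeline, which swings the door open in yaw.
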(event `self.ReceiveBeginPlay`
  (add `self._vaultOpen` (delegate `Open Vault`)))

(event `Open Vault`
  (`/Engine/EditorBlueprintResources/StandardMacros.DoOnce` false
    (:`Completed`
      (bind (_direction _rotation) (`Timeline|Rotating Handle`)
        (:`Update`
          (`SceneComponent.K2_SetRelativeRotation` (`self._pVaultHandle`) (`KismetMathLibrary.MakeRotator` 0.0 (`KismetMathLibrary.Lerp` 0.0 280.0 _rotation)) false false))
        (:`Finished`
          (bind (_direction_2 _rotation_2) (`Timeline|Opening`)
            (:`Update`
              (`SceneComponent.K2_SetRelativeRotation` (`self._pVaultDoor`) (`KismetMathLibrary.MakeRotator` 0.0 0.0 (`KismetMathLibrary.Lerp` 0.0 110.0 _rotation_2)) false false))))))))

(fn `UserConstructionScript`)